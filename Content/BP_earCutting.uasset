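; BP_earCutting is a procedural mesh Blueprint that turns a vertex array into a triangulated mesh, by ear clipping judging by its name.
; The construction script clears the index buffer, refills it through GetIBO from VBO, then creates the mesh section without requesting collision.
; GetIBO's implementation is not included here.
; BeginPlay is empty, and a collision-enabled copy of the build in the event graph is unconnected and never runs.
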(event `self.ReceiveBeginPlay`)

(fn `UserConstructionScript`
  (`KismetArrayLibrary.Array_Clear` (`self.IBO`))
  (bind _ibo (`BFL_EarCutting.GetIBO` (`self.VBO`)))
  (bind _output_get (set `self.IBO` _ibo))
  (`ProceduralMeshComponent.CreateMeshSection_LinearColor` :`self` (`self.ProceduralMesh`) :`Vertices` (`self.VBO`) :`Triangles` _output_get))